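; BP_AudioRecorder is an actor that records captured audio to a WAV file when the R key is pressed.
; Each press toggles an IsRecording flag, calling StartRecording or StopRecording.
; These functions start or stop the AudioCapture component alongside output recording of AudioCaptureSubmix, and print a status string.
; Stopping exports the file as "audio" into a relative record_buffer folder.
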(event EventBeginPlay
  (Variables|Default|SetbIsRecording false))

(event Collision|EventActorBeginOverlap
  (params (OtherActor :type Actor%20Object%20Reference)))

(event EventTick
  (params (DeltaSeconds :type Float%20%28single-precision%29)))

(event Input|KeyboardEvents|R
  (params (Key :type Key%20Structure :default "None"))
  (:Pressed
    (if (Variables|Default|GetbIsRecording)
      (CallFunction|StopRecording)
      (else
        (CallFunction|StartRecording)))))

(fn ConstructionScript)

(fn StopRecording
  (Variables|Default|SetbIsRecording false)
  (Audio|Components|Audio|Stop (Variables|Default|GetAudioCapture))
  (Class|AudioMixerBlueprintLibrary|StopRecordingOutput "WavFile" "audio" "./record_buffer/" "/Game/Submix/AudioCaptureSubmix.AudioCaptureSubmix" 0)
  (Development|PrintString "REC end"))

(fn StartRecording
  (Variables|Default|SetbIsRecording true)
  (CameraShake|Start (Variables|Default|GetAudioCapture))
  (Class|AudioMixerBlueprintLibrary|StartRecordingOutput 1e+01 "/Game/Submix/AudioCaptureSubmix.AudioCaptureSubmix")
  (Development|PrintString "REC start"))