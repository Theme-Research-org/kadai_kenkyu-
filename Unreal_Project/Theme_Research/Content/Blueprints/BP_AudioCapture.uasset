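; BP_AudioCapture is a push-to-talk actor that records audio while R is held and uploads it to AWS through the game mode.
; Pressing R starts recording the SS_AudioCapture submix; releasing it closes the media player and exports recording.wav to the Saved directory.
; After a short delay, MyGameModeBase sends the file, and the completion callback prints the response, deletes the WAV and clears the Recording/Saving guards.
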(event Custom|OnCompleted
  (params (ResponseContent :type String) (bSuccess :type Boolean))
  (Development|PrintString ResponseContent)
  (Class|BlueprintFileUtilsBPLibrary|DeleteFile (Utilities|String|Append (Class|KismetSystemLibrary|GetProjectSavedDirectory) "recording.wav") false false)
  (Variables|Default|SetbRecording false)
  (Variables|Default|SetbSaving false))

(event EventBeginPlay
  (bind _asmy_game_mode_base (Utilities|Casting|CastToMyGameModeBase (Game|GetGameMode)))
  (Variables|Default|SetAs%20My%20Game%20Mode%20Base _asmy_game_mode_base)
  (Input|EnableInput (Game|GetPlayerController 0)))

(event Collision|EventActorBeginOverlap
  (params (OtherActor :type Actor%20Object%20Reference)))

(event EventTick
  (params (DeltaSeconds :type Float%20%28single-precision%29)))

(event Input|KeyboardEvents|R
  (params (Key :type Key%20Structure))
  (bind _mediasound (Variables|Default|GetMediaSound))
  (bind _returnvalue (Class|MediaSoundComponent|GetMediaPlayer _mediasound))
  (:Pressed
    (if (not (Variables|Default|GetbRecording))
      (Variables|Default|SetbRecording true)
      (Class|AudioMixerBlueprintLibrary|StartRecordingOutput 0.0 "/Game/Submixes/SS_AudioCapture.SS_AudioCapture")))
  (:Released
    (if (and (Variables|Default|GetbRecording) (not (Variables|Default|GetbSaving)))
      (Variables|Default|SetbSaving true)
      (if (Class|MediaPlayer|IsClosed _returnvalue)
        _
        (else
          (Media|MediaPlayer|Close _returnvalue :!class /Script/MediaAssets.MediaPlayer)))
      (Class|AudioMixerBlueprintLibrary|StopRecordingOutput "WavFile" "recording" (Class|KismetSystemLibrary|GetProjectSavedDirectory) "/Game/Submixes/SS_AudioCapture.SS_AudioCapture" 0)
      (Utilities|FlowControl|Delay 0.5)
      (Class|MyGameModeBase|SendWavFiletoAWS (Variables|Default|GetAs%20My%20Game%20Mode%20Base) (delegate Custom|OnCompleted)))))

(fn ConstructionScript)